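; Player character Blueprint with hand-built walk, run, turn, dash, jump and fall movement through transform changes.
; Enhanced Input drives MovePlayer, which projects steps onto traced slopes, while timelines animate dash and jump.
; A downward trace each Tick applies constant-speed falling, and capsule hits push physics objects.
; IsJumping and ShouldBlockMoveInput are only set false, SetPlayerRotation is uncalled, and an older dash is disconnected.
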(event OnComponentHit(PlayerCollision)
  (params (HitComponent :type Primitive%20Component%20Object%20Reference) (OtherActor :type Actor%20Object%20Reference) (OtherComp :type Primitive%20Component%20Object%20Reference) (NormalImpulse :type Vector :default "0, 0, 0") (Hit :type Hit%20Result%20Structure%20%28by%20ref%29))
  (if (Physics|IsSimulatingPhysics OtherComp "None")
    (Physics|AddForce OtherComp (* (Math|Vector|GetForwardVector (Variables|Default|GetPlayerMesh)) 5e+02) "None" true)))

(event Input|EnhancedActionEvents|EnhancedInputActionIA_Move
  (params (ActionValue :type Vector%202D%20Structure) (ElapsedSeconds :type Float%20%28double-precision%29) (TriggeredSeconds :type Float%20%28double-precision%29) (InputAction :type Input%20Action%20Object%20Reference :default "/Game/M7/Input/Actions/IA_Move.IA_Move"))
  (if (not (Variables|Default|GetShouldBlockMoveInput))
    (CallFunction|MovePlayer ActionValue)))

(event Input|EnhancedActionEvents|EnhancedInputActionIA_Run
  (params (ActionValue :type Boolean) (ElapsedSeconds :type Float%20%28double-precision%29) (TriggeredSeconds :type Float%20%28double-precision%29) (InputAction :type Input%20Action%20Object%20Reference :default "/Game/M7/Input/Actions/IA_Run.IA_Run"))
  (:Started
    (Variables|Default|SetIsRunning true))
  (:Completed
    (Variables|Default|SetIsRunning false)))

(event Input|EnhancedActionEvents|EnhancedInputActionIA_Jump
  (params (ActionValue :type Boolean) (ElapsedSeconds :type Float%20%28double-precision%29) (TriggeredSeconds :type Float%20%28double-precision%29) (InputAction :type Input%20Action%20Object%20Reference :default "/Game/M7/Input/Actions/IA_Jump.IA_Jump"))
  (bind _returnvalue (Transformation|GetActorLocation))
  (:Started
    (if (and (not (Variables|Default|GetIsJumping)) (not (Variables|Default|GetIsFalling)))
      (Variables|Default|SetIsJumping false)
      (Variables|Default|SetJumpingInitialZ (.z (Transformation|GetActorLocation)))
      (bind _jumpheight (Timeline|JumpCurve PlayFromStart)
        (:Update
          (Transformation|SetActorLocation (Math|Vector|MakeVector (.x _returnvalue) (.y _returnvalue) (+ _jumpheight (Variables|Default|GetJumpingInitialZ))) false false))
        (:Finished
          (Variables|Default|SetIsJumping false))))))

(event Input|EnhancedActionEvents|EnhancedInputActionIA_TurnLeft
  (params (ActionValue :type Vector%202D%20Structure) (ElapsedSeconds :type Float%20%28double-precision%29) (TriggeredSeconds :type Float%20%28double-precision%29) (InputAction :type Input%20Action%20Object%20Reference :default "/Game/M7/Input/Actions/IA_TurnLeft.IA_TurnLeft"))
  (Class|Actor|AddActorWorldRotation (Math|Rotator|MakeRotator 0.0 0.0 (* (Utilities|Time|GetWorldDeltaSeconds) -6e+01)) true))

(event Input|EnhancedActionEvents|EnhancedInputActionIA_TurnRight
  (params (ActionValue :type Vector%202D%20Structure) (ElapsedSeconds :type Float%20%28double-precision%29) (TriggeredSeconds :type Float%20%28double-precision%29) (InputAction :type Input%20Action%20Object%20Reference :default "/Game/M7/Input/Actions/IA_TurnRight.IA_TurnRight"))
  (Class|Actor|AddActorWorldRotation (Math|Rotator|MakeRotator 0.0 0.0 (* (Utilities|Time|GetWorldDeltaSeconds) 6e+01)) true))

(event Input|EnhancedActionEvents|EnhancedInputActionIA_Dash
  (params (ActionValue :type Boolean) (ElapsedSeconds :type Float%20%28double-precision%29) (TriggeredSeconds :type Float%20%28double-precision%29) (InputAction :type Input%20Action%20Object%20Reference :default "/Game/M7/Input/Actions/IA_Dash.IA_Dash"))
  (bind _returnvalue (Transformation|GetVelocity))
  (:Started
    (Variables|Default|SetShouldBlockMoveInput false)
    (Variables|Default|SetInitialDashPosition (Transformation|GetActorLocation))
    (bind _dashdistance (Timeline|Dash PlayFromStart)
      (:Update
        (Transformation|SetActorLocation (+ (Variables|Default|GetInitialDashPosition) (* (select (> (Math|Vector|VectorLength _returnvalue) 0.0) _returnvalue (Math|Vector|GetForwardVector (Variables|Default|GetPlayerMesh))) _dashdistance)) true false))
      (:Finished
        (Variables|Default|SetShouldBlockMoveInput false)))))

(event EventTick
  (params (DeltaSeconds :type Float%20%28single-precision%29))
  (bind _returnvalue (Transformation|GetActorLocation))
  (bind _playercollision (Variables|Default|GetPlayerCollision))
  (bind _returnvalue_2 (Components|Capsule|GetScaledCapsuleHalfHeight _playercollision))
  (bind _returnvalue_3 (- (.z _returnvalue) _returnvalue_2))
  (bind _returnvalue_4 (Collision|MultiLineTraceByChannel (Math|Vector|MakeVector (.x _returnvalue) (.y _returnvalue) _returnvalue_3) (Math|Vector|MakeVector (.x _returnvalue) (.y _returnvalue) (- _returnvalue_3 2e+01)) "TraceTypeQuery1" false 0 "None"))
  (bind _output_get (Variables|Default|SetIsFalling (not _returnvalue_4)))
  (if (and _output_get (not (Variables|Default|GetIsJumping)))
    (Transformation|AddActorWorldOffset (Math|Vector|MakeVector 0.0 0.0 (* (Variables|Default|GetFallingVelocity) (Utilities|Time|GetWorldDeltaSeconds))) true)))

(fn ConstructionScript)

(fn SetPlayerRotation
  (params (X :type Float%20%28double-precision%29) (Y :type Float%20%28double-precision%29))
  (bind _returnvalue (Transformation|GetActorLocation))
  (Transformation|SetRelativeRotation (Variables|Default|GetPlayerMesh) (Math|Rotator|FindLookatRotation _returnvalue (+ (* (Transformation|GetActorForwardVector) Y) (* (Transformation|GetActorRightVector) X) _returnvalue)) false false))

(fn MovePlayer
  (params (InputVector :type Vector%202D%20Structure))
  (bind _returnvalue (Utilities|Time|GetWorldDeltaSeconds))
  (bind _isrunning (Variables|Default|GetIsRunning))
  (bind _walkingvelocity (Variables|Default|GetWalkingVelocity))
  (bind _runningvelocity (Variables|Default|GetRunningVelocity))
  (bind _returnvalue_2 (select _isrunning _runningvelocity _walkingvelocity))
  (bind _returnvalue_3 (* _returnvalue _returnvalue_2))
  (bind _returnvalue_4 (* InputVector _returnvalue_3))
  (bind _returnvalue_5 (Math|Vector|MakeVector (.y _returnvalue_4) (.x _returnvalue_4) 0.0))
  (LocalVariables|SetBasicMovementVector (+ (* (Transformation|GetActorForwardVector) (.x _returnvalue_5)) (* (.y _returnvalue_5) (Transformation|GetActorRightVector))))
  (bind (_outhit _returnvalue_6) (Collision|LineTraceByChannel (+ (Transformation|GetActorLocation) (* (LocalVariables|GetBasicMovementVector) 2e+01)) (- (+ (Transformation|GetActorLocation) (* (LocalVariables|GetBasicMovementVector) 2e+01)) "0.000000,0.000000,200.000000") "TraceTypeQuery1" false 0 "None"))
  (Transformation|AddActorWorldOffset (select _returnvalue_6 (Math|Vector|ProjectVectorontoPlane (LocalVariables|GetBasicMovementVector) (.impactnormal _outhit)) (LocalVariables|GetBasicMovementVector)) true))