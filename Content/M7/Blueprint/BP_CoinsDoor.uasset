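; A door actor that opens once the player has collected every BP_Coin in the level.
; On BeginPlay it gathers all coins, binds their pickup events to a counter and compares it to the total.
; When the last coin is taken, it disables player input and blends the camera to the door, then a timeline slides the blade along two axes.
; Afterwards the view blends back to the pawn and input returns.
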(event Custom|OpenDoor
  (Input|DisableInput (Game|Player|GetPlayerPawn 0) (Game|GetPlayerController 0))
  (Game|Player|SetViewTargetwithBlend (Game|GetPlayerController 0) self 2.0 "VTBlend_EaseInOut" 1.0 false)
  (Utilities|FlowControl|Delay 3.0)
  (bind (_direction _vertical_movement _depth_movement) (Timeline|Opening%20Animation PlayFromStart)
    (:Update
      (Transformation|SetRelativeLocation (Variables|Default|GetDoorBlade) (Math|Vector|MakeVector _depth_movement 0.0 _vertical_movement) false false))
    (:Finished
      (Utilities|FlowControl|Delay 2.0)
      (Game|Player|SetViewTargetwithBlend (Game|GetPlayerController 0) (Game|Player|GetPlayerPawn 0) 1.0 "VTBlend_EaseInOut" 1.0 false)
      (Utilities|FlowControl|Delay 1.0)
      (Input|EnableInput (Game|Player|GetPlayerPawn 0) (Game|GetPlayerController 0)))))

(event Custom|IncreaseCoinCounter
  (Math|Integer|IncrementInt (Variables|Default|GetCoinsCollected)
    (:%20%20
      (if (>= (Variables|Default|GetCoinsCollected) (Variables|Default|GetCoinsToCollect))
        (CallFunction|OpenDoor)))))

(event EventBeginPlay
  (bind _outactors (Actor|GetAllActorsOfClass "/Game/M7/Blueprint/BP_Coin.BP_Coin_C"))
  (bind _output_get (Variables|Default|SetCoinReferences _outactors))
  (Variables|Default|SetCoinsToCollect (Utilities|Array|Length _output_get))
  (for _array_element (Variables|Default|GetCoinReferences)
    (EventDispatchers|BindEventtoOnCoinPickUp _array_element (delegate Custom|IncreaseCoinCounter))))

(fn ConstructionScript)